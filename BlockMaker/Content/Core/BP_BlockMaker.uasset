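; BP_BlockMaker is an actor that builds a wall-like grid of half-scale static mesh blocks when play begins.
; Nested loops over the height and width counts add one component per cell, spaced along local Z and Y by SpaceBetween.
; The blocks are components of this actor rather than separate actors, and the construction script is empty, so the grid is created only at runtime.
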(event `self.ReceiveBeginPlay`
  (for _index (range 1 (+ (`self.HowManyBlocksTall`) 1))
    (for _index_2 (range 1 (+ (`self.HowManyBlocksWide`) 1))
      (`AddComponent|NODE_AddStaticMeshComponent-0` :`RelativeTransform` (`KismetMathLibrary.MakeTransform` (`KismetMathLibrary.MakeVector` 0.0 (`KismetMathLibrary.Conv_IntToDouble` (* _index_2 (`self.SpaceBetween`))) (`KismetMathLibrary.Conv_IntToDouble` (* _index (`self.SpaceBetween`)))) (struct) (0.5 0.5 0.5))))))

(fn `UserConstructionScript`)