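; Room actor for a text adventure that rebuilds itself from room data.
; DisplayRoom clears the previous interactibles, positions four child wall builders by room width and depth, then builds each wall.
; It spawns interactibles by mapped room location, though only North has a computed position.
; ShowHiddenItem spawns the room's collectible into ActiveCollectibles, which Cleanup does not clear.
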(event `self.ReceiveBeginPlay`)

(fn `Cleanup`
  (bind _visiblehiddeniteminroom (`self.visibleHiddenItemInRoom`))
  ;[1 1 1] Remove (hidden) static meshes
  (`/Engine/EditorBlueprintResources/StandardMacros.IsValid` _visiblehiddeniteminroom
    (:`Is Valid`
      (`self.K2_DestroyActor` _visiblehiddeniteminroom))
    (:`Is Not Valid`
      _))
  ;[1 1 1] Clean up any interactibles
  (bind _values (`BlueprintMapLibrary.Map_Values` (`self.ActiveInteractibles`)))
  (for _array_element _values
    (`self.K2_DestroyActor` _array_element))
  (`BlueprintMapLibrary.Map_Clear` (`self.ActiveInteractibles`)))

(fn `DisplayRoom`
  (params (RoomData :type "/Game/TextAdventure/Core/DS_RoomData Structure"))
  (bind _north (`self.North`))
  (bind _south (`self.South`))
  (bind _west (`self.West`))
  (bind _east (`self.East`))
  (bind (_iteminroom _northwall _eastwall _southwall) (break `/Game/TextAdventure/Core/DS_RoomData` (`self.ActiveRoomData`)))
  (bind (_iteminroom_2 _northwall_2 _eastwall_2 _southwall_2 _westwall _basicdescription _searchstrings _roomwidth _roomheight _roomdepth) (break `/Game/TextAdventure/Core/DS_RoomData` (`self.ActiveRoomData`)))
  (bind (_iteminroom_3 _northwall_3 _eastwall_3 _southwall_3 _westwall_2 _basicdescription_2 _searchstrings_2 _roomwidth_2 _roomheight_2 _roomdepth_2 _interactiblesinroom) (break `/Game/TextAdventure/Core/DS_RoomData` (`self.ActiveRoomData`)))
  (`self.Cleanup`)
  (bind _output_get (set `self.ActiveRoomData` RoomData))
  (`|ExecutionSequence`
    (:`then_0`
      (bind (_iteminroom_4 _northwall_4 _eastwall_4 _southwall_4 _westwall_3 _basicdescription_3 _searchstrings_3 _roomwidth_3 _roomheight_3 _roomdepth_3) (break `/Game/TextAdventure/Core/DS_RoomData` _output_get))
      (bind _returnvalue (/ _roomdepth_3 2.0))
      (`SceneComponent.K2_SetRelativeLocation` _south (`KismetMathLibrary.MakeVector` 0.0 _returnvalue) false false)
      (`SceneComponent.K2_SetRelativeLocation` _north (`KismetMathLibrary.MakeVector` 0.0 (* _returnvalue -1.0)) false false)
      (`/Game/TextAdventure/Core/BP_WallBuilder.BuildWall` (cast `/Game/TextAdventure/Core/BP_WallBuilder` (`ChildActorComponent.ChildActor` _north) :!pure true) _northwall _roomwidth_3 _roomheight_3)
      (`/Game/TextAdventure/Core/BP_WallBuilder.BuildWall` (cast `/Game/TextAdventure/Core/BP_WallBuilder` (`ChildActorComponent.ChildActor` _south) :!pure true) _southwall _roomwidth_3 _roomheight_3))
    (:`then_1`
      (bind _returnvalue_2 (/ _roomwidth_3 2.0))
      (`SceneComponent.K2_SetRelativeLocation` _west (`KismetMathLibrary.MakeVector` (* _returnvalue_2 -1.0)) false false)
      (`SceneComponent.K2_SetRelativeLocation` _east (`KismetMathLibrary.MakeVector` _returnvalue_2) false false)
      (`/Game/TextAdventure/Core/BP_WallBuilder.BuildWall` (cast `/Game/TextAdventure/Core/BP_WallBuilder` (`ChildActorComponent.ChildActor` _east) :!pure true) _eastwall_2 _roomdepth _roomheight)
      (`/Game/TextAdventure/Core/BP_WallBuilder.BuildWall` (cast `/Game/TextAdventure/Core/BP_WallBuilder` (`ChildActorComponent.ChildActor` _west) :!pure true) _westwall _roomdepth _roomheight))
    (:`then_2`
      (bind _keys (`BlueprintMapLibrary.Map_Keys` _interactiblesinroom))
      (for _array_element _keys
        (`self.PlaceInteractible` (`BlueprintMapLibrary.Map_Find` _interactiblesinroom _array_element) _array_element)))))

(fn `PlaceInteractible`
  (params (Interactible :type "/Game/TextAdventure/Interactibles/DS_Interactible Structure") (Location :type "/Game/TextAdventure/Interactibles/EPositionInRoom Enum" :default "NewEnumerator0"))
  (locals (PercentagePlacement :type "Float (double-precision)" :default 0.8) (InteractiblePosition :type "Vector Structure"))
  (bind _returnvalue (`self.RoomLocationToWorldLocation` Location))
  (bind _returnvalue_2 (`|SpawnActorFromClass` "/Game/TextAdventure/Core/BP_Interactible.BP_Interactible_C" _returnvalue "Undefined" "OverrideRootScale" null Interactible null))
  (`BlueprintMapLibrary.Map_Add` (`self.ActiveInteractibles`) Location _returnvalue_2))

(fn `RoomLocationToWorldLocation`
  (params (Selection :type "/Game/TextAdventure/Interactibles/EPositionInRoom Enum" :default "NewEnumerator0"))
  (returns (ReturnValue :type "Transform Structure"))
  (locals (PercentagePlacement :type "Float (double-precision)" :default 0.8) (InteractiblePosition :type "Vector Structure"))
  (switch `/Game/TextAdventure/Interactibles/EPositionInRoom` Selection
    (:`NewEnumerator1`
      (bind _output_get (set `local.InteractiblePosition` (`KismetMathLibrary.MakeVector` 0.0 (* (`.RoomDepth_46_A896A5124110732BF5A76F8C7F8A7334` (break `/Game/TextAdventure/Core/DS_RoomData` (`self.ActiveRoomData`))) 0.5 (`local.PercentagePlacement`) -1.0))))
      (return (`KismetMathLibrary.Conv_VectorToTransform` _output_get)))))

(fn `ShowHiddenItem`
  (locals (itemLocation :type "Transform Structure" :default "0.000000,0.000000,2.000000|0.000000,0.000000,0.000000|1.000000,1.000000,1.000000"))
  (bind _returnvalue (`|SpawnActorFromClass` "/Game/TextAdventure/Collectibles/BP_Collectible.BP_Collectible_C" (`local.itemLocation`) "Undefined" "OverrideRootScale" null (`.ItemInRoom_49_0C2FCD3542A82ED5C5CF40904021FA77` (break `/Game/TextAdventure/Core/DS_RoomData` (`self.ActiveRoomData`))) null))
  (`BlueprintMapLibrary.Map_Add` (`self.ActiveCollectibles`) "NewEnumerator8" _returnvalue))

(fn `UserConstructionScript`)