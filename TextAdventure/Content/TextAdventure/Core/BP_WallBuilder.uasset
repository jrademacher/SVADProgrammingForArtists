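; Procedural wall actor for the text adventure that assembles a wall, with an optional doorway, from scaled static mesh components.
; BuildWall takes wall data and size, destroys the previous pieces, derives offsets in InitializeVariables, then adds and tracks new meshes.
; The door destination selects two side panels plus lintel or one solid panel, always capped by an upper section.
; The construction script calls BuildWall with zero size and retains an older, disconnected copy of the logic.
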(fn `BuildWall`
  (params (WallData :type "/Game/TextAdventure/Core/DS_WallData Structure") (WallWidth :type "Float (double-precision)") (WallHeight :type "Float (double-precision)"))
  (bind (_activewalldata_door_destination _activewalldata_door_width _activewalldata_door_height) (break `/Game/TextAdventure/Core/DS_WallData` (`self.ActiveWallData`)))
  (bind (_activewalldata_door_destination_2 _activewalldata_door_width_2 _activewalldata_door_height_2) (break `/Game/TextAdventure/Core/DS_WallData` (`self.ActiveWallData`)))
  (bind (_activewalldata_door_destination_3 _activewalldata_door_width_3 _activewalldata_door_height_3) (break `/Game/TextAdventure/Core/DS_WallData` (`self.ActiveWallData`)))
  (bind _returnvalue (- (`self.WallHeight`) _activewalldata_door_height_3))
  (bind _returnvalue_2 (+ (`self.HalfDoor`) (`self.HalfWallMidpoint`)))
  (`ActorComponent.K2_DestroyComponent` (`self.WallList`))
  (set `self.WallHeight` WallHeight)
  (set `self.WallWidth` WallWidth)
  (set `self.ActiveWallData` WallData)
  (`self.InitializeVariables`)
  ;[1 1 1] Do we have a door?
  (if (`|EnumInequality` (`.Door_Destination_14_7D5D9DDB496010598C4253AE894CF7F6` (break `/Game/TextAdventure/Core/DS_WallData` (`self.ActiveWallData`))) "NewEnumerator0")
    (bind _returnvalue_3 (`AddComponent|NODE_AddStaticMeshComponent-11` :`RelativeTransform` (`KismetMathLibrary.MakeTransform` (`KismetMathLibrary.MakeVector` (* _returnvalue_2 -1.0) 0.0 (`self.HalfDoorHeight`)) (struct) (`KismetMathLibrary.MakeVector` (`self.HalfWall`) 1.0 _activewalldata_door_height))))
    (`KismetArrayLibrary.Array_Add` (`self.WallList`) _returnvalue_3)
    (bind _returnvalue_4 (`AddComponent|NODE_AddStaticMeshComponent-12` :`RelativeTransform` (`KismetMathLibrary.MakeTransform` (`KismetMathLibrary.MakeVector` _returnvalue_2 0.0 (`self.HalfDoorHeight`)) (struct) (`KismetMathLibrary.MakeVector` (`self.HalfWall`) 1.0 _activewalldata_door_height))))
    (`KismetArrayLibrary.Array_Add` (`self.WallList`) _returnvalue_4)
    ;[1 1 1] Lintel
    (bind _returnvalue_5 (`AddComponent|NODE_AddStaticMeshComponent-15` :`RelativeTransform` (`KismetMathLibrary.MakeTransform` (`KismetMathLibrary.MakeVector` 0.0 0.0 (+ _activewalldata_door_height_2 1.0)) (struct) (`KismetMathLibrary.MakeVector` _activewalldata_door_width_2 4.0 2.0))))
    (`KismetArrayLibrary.Array_Add` (`self.WallList`) _returnvalue_5)
    (else
      (bind _returnvalue_6 (`AddComponent|NODE_AddStaticMeshComponent-14` :`RelativeTransform` (`KismetMathLibrary.MakeTransform` (`KismetMathLibrary.MakeVector` 0.0 0.0 (`self.HalfDoorHeight`)) (struct) (`KismetMathLibrary.MakeVector` (`self.WallWidth`) 1.0 _activewalldata_door_height))))
      (`KismetArrayLibrary.Array_Add` (`self.WallList`) _returnvalue_6)))
  ;[1 1 1] Top portion of the wall
  (bind _returnvalue_7 (`AddComponent|NODE_AddStaticMeshComponent-13` :`RelativeTransform` (`KismetMathLibrary.MakeTransform` (`KismetMathLibrary.MakeVector` 0.0 0.0 (+ (/ _returnvalue 2.0) _activewalldata_door_height_3)) (struct) (`KismetMathLibrary.MakeVector` (`self.WallWidth`) 1.0 _returnvalue))))
  (`KismetArrayLibrary.Array_Add` (`self.WallList`) _returnvalue_7))

(fn `InitializeVariables`
  (bind ((`Door_Width_6_CD88038C419A699532AEA3B7258E6F7C` _door_width)) (break `/Game/TextAdventure/Core/DS_WallData` (`self.ActiveWallData`)))
  (set `self.HalfDoor` (/ _door_width 2.0))
  (bind _output_get (set `self.HalfWall` (/ (- (`self.WallWidth`) _door_width) 2.0)))
  (set `self.HalfDoorHeight` (/ (`.Door_Height_10_56832CC9434CE0847E4722BB843E5250` (break `/Game/TextAdventure/Core/DS_WallData` (`self.ActiveWallData`))) 2.0))
  (set `self.HalfWallMidpoint` (/ _output_get 2.0)))

(fn `UserConstructionScript`
  (`self.BuildWall` (`self.ActiveWallData`)))