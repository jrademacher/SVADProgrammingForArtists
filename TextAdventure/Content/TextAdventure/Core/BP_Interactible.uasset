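; BP_Interactible is a text-adventure world object that changes when clicked with the required item selected.
; Its data struct drives the construction script, which picks the pre- or post-interaction mesh.
; Releasing a click on the mesh compares the required item to RoomNav's selected item, then on a match marks it interacted, swaps mesh and displays a message.
; Collectible spawning nodes exist but are unconnected.
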(event `self.InteractibleMesh.OnReleased`
  (params (TouchedComponent :type "PrimitiveComponent Object Reference") (ButtonReleased :type "Key Structure"))
  (`self.interactedWith`))

(fn `buildSelf`
  (params (WhoAmI :type "/Game/TextAdventure/Interactibles/DS_Interactible Structure"))
  (bind _output_get (set `self.infoAboutInteractible` WhoAmI))
  (bind (_preinteractmesh _postinteractmesh _spawns _needsitemselected _destroyinventoryitemused _messagetodisplayafterinteraction _hasbeeninteractedwith) (break `/Game/TextAdventure/Interactibles/DS_Interactible` _output_get))
  (`StaticMeshComponent.SetStaticMesh` (`self.InteractibleMesh`) (select `bool` _hasbeeninteractedwith :`false` _preinteractmesh :`true` _postinteractmesh)))

(fn `interactedWith`
  (bind (_preinteractmesh _postinteractmesh _spawns _needsitemselected _destroyinventoryitemused _messagetodisplayafterinteraction) (break `/Game/TextAdventure/Interactibles/DS_Interactible` (`self.infoAboutInteractible`)))
  (if (`|EnumEquality` _needsitemselected (`/Game/TextAdventure/Core/WP_RoomNav.selectedItem` (`/Game/TextAdventure/Core/GM_TextAdventure.RoomNav` (cast `/Game/TextAdventure/Core/GM_TextAdventure` (`GameplayStatics.GetGameMode`) :!pure true))))
    (bind _structout (setmembers `/Game/TextAdventure/Interactibles/DS_Interactible` :`StructRef` (`self.infoAboutInteractible`) :`HasBeenInteractedWith` true))
    (set `self.infoAboutInteractible` _structout)
    (`StaticMeshComponent.SetStaticMesh` (`self.InteractibleMesh`) _postinteractmesh)
    (`/Game/TextAdventure/Core/BPFL_DataHelpers.DisplayMessage` _messagetodisplayafterinteraction)))

(fn `UserConstructionScript`
  (`self.buildSelf` (`self.infoAboutInteractible`)))