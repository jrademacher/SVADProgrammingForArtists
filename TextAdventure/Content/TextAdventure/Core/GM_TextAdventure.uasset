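; Game mode for a text adventure that tracks the current room and the inventory.
; On BeginPlay it loads the starting room from DT_RoomData by enum name, displays it in a spawned BP_Room and adds the WP_RoomNav widget.
; GoInDirection follows the chosen wall's door destination to redisplay that same room actor with new row data.
; It also reveals hidden items on search and fires an inventory-change dispatcher on adds and successful removals.
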(event `self.ReceiveBeginPlay`
  (bind _output_get (set `self.CurrentRoomName` "NewEnumerator1"))
  (bind _returnvalue (`|GetDataTableRow` "/Game/TextAdventure/Core/DT_RoomData.DT_RoomData" (`KismetStringLibrary.Conv_StringToName` (`|GetEnumeratorNameAsString` _output_get)))
    (:`then`
      (bind _output_get_2 (set `self.CurrentRoomData` _returnvalue))
      (bind _returnvalue_2 (`|SpawnActorFromClass` "/Game/TextAdventure/Core/BP_Room.BP_Room_C" (`self.zeroLOC`) "Undefined" "OverrideRootScale" null null))
      (set `self.CurrentRoom` _returnvalue_2)
      (`/Game/TextAdventure/Core/BP_Room.DisplayRoom` _returnvalue_2 _output_get_2)
      (bind _returnvalue_3 (`|CreateWidget` "/Game/TextAdventure/Core/WP_RoomNav.WP_RoomNav_C"))
      (`UserWidget.AddToViewport` _returnvalue_3 0)
      (set `self.RoomNav` _returnvalue_3))))

(fn `AddItemToInventory`
  (params (incomingItem :type "/Game/TextAdventure/Collectibles/ECollectibleTypes Enum (by ref)" :default "NewEnumerator2"))
  (`KismetArrayLibrary.Array_Add` (`self.Inventory`) incomingItem)
  (`self.OnInventoryChange`))

(fn `GoInDirection`
  (params (directionInput :type "/Game/TextAdventure/Core/EDirection Enum" :default "NewEnumerator0"))
  (locals (PotentialDestination :type "/Game/TextAdventure/Core/ERoomTypes Enum"))
  (bind (_iteminroom _northwall _eastwall _southwall _westwall) (break `/Game/TextAdventure/Core/DS_RoomData` (`self.CurrentRoomData`)))
  (bind _door_destination (break `/Game/TextAdventure/Core/DS_WallData` (select `/Game/TextAdventure/Core/EDirection` directionInput :`NewEnumerator0` _northwall :`NewEnumerator1` _eastwall :`NewEnumerator2` _southwall :`NewEnumerator3` _westwall)))
  (bind _returnvalue (`|GetEnumeratorNameAsString` _door_destination))
  (bind _output_get (set `local.PotentialDestination` _door_destination))
  (if (`|EnumInequality` _output_get "NewEnumerator0")
    (`KismetSystemLibrary.PrintString` _returnvalue)
    (bind _returnvalue_2 (`|GetDataTableRow` "/Game/TextAdventure/Core/DT_RoomData.DT_RoomData" (`KismetStringLibrary.Conv_StringToName` _returnvalue))
      (:`then`
        (`/Game/TextAdventure/Core/BP_Room.DisplayRoom` (`self.CurrentRoom`) _returnvalue_2)
        (set `self.CurrentRoomData` _returnvalue_2)
        (set `self.CurrentRoomName` (`local.PotentialDestination`))))))

(fn `RemoveItemFromInventory`
  (params (Item :type "/Game/TextAdventure/Collectibles/ECollectibleTypes Enum (by ref)" :default "NewEnumerator2"))
  (bind _returnvalue (`KismetArrayLibrary.Array_RemoveItem` (`self.Inventory`) Item))
  (if _returnvalue
    (`self.OnInventoryChange`)))

(fn `SearchCurrentRoom`
  (`/Game/TextAdventure/Core/BP_Room.ShowHiddenItem` (`self.CurrentRoom`)))

(fn `UserConstructionScript`)