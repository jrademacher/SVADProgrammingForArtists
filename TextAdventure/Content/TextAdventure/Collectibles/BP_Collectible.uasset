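; BP_Collectible is a pickup actor for the text adventure game, representing one item type chosen by CollectibleType.
; The construction script calls BuildSelf, which stores the type and sets the static mesh from that type's item data lookup.
; When the mesh receives an OnReleased click event, it adds the type to the inventory through GM_TextAdventure and destroys itself.
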(event `self.ReceiveBeginPlay`)

(event `self.StaticMesh.OnReleased`
  (params (TouchedComponent :type "PrimitiveComponent Object Reference") (ButtonReleased :type "Key Structure"))
  (`/Game/TextAdventure/Core/GM_TextAdventure.AddItemToInventory` (cast `/Game/TextAdventure/Core/GM_TextAdventure` (`GameplayStatics.GetGameMode`) :!pure true) (`self.CollectibleType`))
  (`self.K2_DestroyActor`))

(fn `buildSelf`
  (params (TypeToBuild :type "/Game/TextAdventure/Collectibles/ECollectibleTypes Enum" :default "NewEnumerator2"))
  (bind _output_get (set `self.CollectibleType` TypeToBuild))
  (`StaticMeshComponent.SetStaticMesh` (`self.StaticMesh`) (`.Mesh_2_62CF45DA44F39225486FEB97906E33A6` (break `/Game/TextAdventure/Core/DS_Item` (`/Game/TextAdventure/Core/BPFL_DataHelpers.GivenEnumGetItemData` _output_get)))))

(fn `UserConstructionScript`
  (`self.buildSelf` (`self.CollectibleType`)))